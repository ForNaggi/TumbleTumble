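; BP_DoorEX is a two-panel door gimmick that opens once enough pressure switches are active.
; Server-named activate and deactivate events call multicast-named events, which raise or lower the active switch count and compare it to the required number.
; Two timelines then play, or reverse when below the threshold, each sliding one panel along its relative Y axis.
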(event `Multicast_PlayDoorTimeline`
  (`/Engine/EditorBlueprintResources/StandardMacros.IncrementInt` (`self.PressureSwitchesActive`)
    (:`  `
      (if (>= (`self.PressureSwitchesActive`) (`self.PressureSwitchesNeeded`))
        (`|ExecutionSequence`
          (:`then_0`
            (bind (_direction _doorposition) (`Timeline|DoorActivation` :!label _label)
              (:`Update`
                (`SceneComponent.K2_SetRelativeLocation` (`self.DoorOposite`) (`KismetMathLibrary.MakeVector` 0.0 _doorposition) false false))))
          (:`then_1`
            (bind (_direction_2 `_새_트랙_0`) (`Timeline|DoorOppositeAActivate` :!label _label_2)
              (:`Update`
                (`SceneComponent.K2_SetRelativeLocation` (`self.Door`) (`KismetMathLibrary.MakeVector` 0.0 `_새_트랙_0`) false false)))))
        (else
          (`|ExecutionSequence`
            (:`then_0`
              (goto _label :!via `Reverse`))
            (:`then_1`
              (goto _label_2 :!via `Reverse`))))))))

(event `Multicast_DePlayDoorTimeline`
  (`/Engine/EditorBlueprintResources/StandardMacros.DecrementInt` (`self.PressureSwitchesActive`)
    (:`  `
      (if (>= (`self.PressureSwitchesActive`) (`self.PressureSwitchesNeeded`))
        (`|ExecutionSequence`
          (:`then_0`
            (goto _label))
          (:`then_1`
            (goto _label_2)))
        (else
          (`|ExecutionSequence`
            (:`then_0`
              (goto _label :!via `Reverse`))
            (:`then_1`
              (goto _label_2 :!via `Reverse`))))))))

(event `Server_ActivateDoor`
  (`self.Multicast_PlayDoorTimeline`))

(event `Server_DeActivateDoor`
  (`self.Multicast_DePlayDoorTimeline`))

(fn `UserConstructionScript`)