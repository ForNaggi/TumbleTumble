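; Actor component that gives a character physical-animation ragdolling, switching between optional active ragdoll while walking and full-body ragdoll.
; SetRagdoll receives the components and bones; walking mode simulates bodies below the given bone, keeping feet animated.
; Tick triggers full ragdoll when a downward trace finds no ground, then moves the capsule with the body.
; StandUp saves a pose snapshot, picks a front or back get-up montage by sphere trace, and reattaches the mesh.
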(event `SetRagdoll`
  (params (`Skeletal Mesh` :type "SkeletalMeshComponent Object Reference") (`Capsule Component` :type "CapsuleComponent Object Reference") (`Socket Name` :type Name) (PhysicalAnimationComponent :type "PhysicalAnimationComponent Object Reference") (RightFoot :type Name) (LeftFoot :type Name) (`CharacterMovement ` :type "CharacterMovementComponent Object Reference") (`Always use Active Ragdoll` :type Boolean :default true))
  ;[0.09412 0.09412 0.09412] Set Variables And Components
  (set `self.Mesh` `Skeletal Mesh`)
  (set `self.CapsuleComponent` `Capsule Component`)
  (set `self.Relative Transform` (`SceneComponent.GetRelativeTransform` `Skeletal Mesh`))
  (set `self.Socket Name` `Socket Name`)
  (bind _output_get (set `self.Physical Animation Component` PhysicalAnimationComponent))
  (`PhysicalAnimationComponent.SetSkeletalMeshComponent` _output_get (`self.Mesh`))
  (set `self.RightFoot` RightFoot)
  (set `self.LeftFoot` LeftFoot)
  (set `self.Character Movement` `CharacterMovement `)
  (set `self.Use Active Ragdoll When Walking` `Always use Active Ragdoll`)
  (`self.NormalWalkingRagdoll`))

(event `self.ReceiveTick`
  (params (DeltaSeconds :type "Float (single-precision)"))
  (bind _mesh (`self.Mesh`))
  (bind (_returnvalue_x _returnvalue_y _returnvalue_z) (`KismetMathLibrary.BreakVector` (`SceneComponent.K2_GetComponentLocation` _mesh)))
  ;[0.09412 0.09412 0.09412] Move Capsule To Body
  (set `self.Delta Seconds` DeltaSeconds)
  (if (`self.Ragdoll`)
    (if (not (`self.CanMove`))
      (`SceneComponent.K2_SetWorldLocation` (`self.CapsuleComponent`) (`SceneComponent.GetSocketLocation` (`self.Mesh`) (`self.Socket Name`)) false false))
    (else
      ;[0.09412 0.09412 0.09412] Check Height
      (bind (_outhit _returnvalue) (`KismetSystemLibrary.LineTraceSingle` (`SceneComponent.K2_GetComponentLocation` _mesh) (`KismetMathLibrary.MakeVector` _returnvalue_x _returnvalue_y (- _returnvalue_z (`self.Height For Ragdoll`))) "TraceTypeQuery1"))
      (if (not _returnvalue)
        (`self.ActivateRagdoll`)))))

(event `NormalWalkingRagdoll`
  (bind _socket_name (`self.Socket Name`))
  (bind _mesh (`self.Mesh`))
  ;[0.09412 0.09412 0.09412] Normal Walking Ragdoll
  (if (`self.Use Active Ragdoll When Walking`)
    (`PhysicalAnimationComponent.ApplyPhysicalAnimationSettingsBelow` (`self.Physical Animation Component`) _socket_name (make `PhysicalAnimationData` true 1000.0 700.0 700.0 700.0) true)
    (`SkeletalMeshComponent.SetAllBodiesBelowSimulatePhysics` _mesh _socket_name true false)
    (`SkeletalMeshComponent.SetAllBodiesBelowSimulatePhysics` _mesh (`self.LeftFoot`) false true)
    (`SkeletalMeshComponent.SetAllBodiesBelowSimulatePhysics` _mesh (`self.RightFoot`) false true)))

(event `ActivateRagdoll`
  ;[0.09412 0.09412 0.09412] Activate Full Body Ragdoll
  (if (not (`self.Ragdoll`))
    (`PhysicalAnimationComponent.ApplyPhysicalAnimationSettingsBelow` (`self.Physical Animation Component`) (`self.Socket Name`) (make `PhysicalAnimationData` true 0.0 300.0 300.0 300.0) true)
    (`SkeletalMeshComponent.SetAllBodiesSimulatePhysics` (`self.Mesh`) true)
    (set `self.Ragdoll` true)
    (set `self.CanMove` false)))

(event `StandUp`
  (bind _mesh (`self.Mesh`))
  (bind _returnvalue (`SceneComponent.GetSocketLocation` (`self.Mesh`) (`self.Socket Name`)))
  ;[0.09412 0.09412 0.09412] Stand Up
  (if (`NavMovementComponent.IsFalling` (`self.Character Movement`))
    _
    (elif (`self.Ragdoll`)
      (`AnimInstance.SavePoseSnapshot` (`SkeletalMeshComponent.GetAnimInstance` (`self.Mesh`)) "Ragdoll")
      (bind (_outhit _returnvalue_2) (`KismetSystemLibrary.SphereTraceSingle` _returnvalue (+ _returnvalue (* (`KismetMathLibrary.GetUpVector` (`SceneComponent.GetSocketRotation` (`self.Mesh`) (`self.Socket Name`))) 50.0)) 5.0 "TraceTypeQuery1"))
      (if _returnvalue_2
        (`|PlayMontage` (`self.Mesh`) (`self.Getting Up Animation Front`)
          (:`then`
            (set `self.Ragdoll` false :!label _label)
            (`SceneComponent.K2_AttachToComponent` _mesh (`self.CapsuleComponent`) (`self.Socket Name`) "SnapToTarget" "SnapToTarget" "SnapToTarget" true)
            (`SceneComponent.K2_SetRelativeTransform` _mesh (`self.Relative Transform`) false false)
            (`self.NormalWalkingRagdoll`))
          (:`OnBlendOut`
            (if (not (`self.Ragdoll`)) :!label _label_2
              (set `self.CanMove` true)))
          (:`OnInterrupted`
            (goto _label_2)))
        (else
          (`|PlayMontage` (`self.Mesh`) (`self.Getting Up Animation Back`)
            (:`then`
              (goto _label))
            (:`OnBlendOut`
              (goto _label_2))
            (:`OnInterrupted`
              (goto _label_2))))))))